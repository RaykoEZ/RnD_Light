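; DistantTest_BP is a distance test actor that moves a Landcruiser cylinder mesh along world Y relative to its camera.
; On BeginPlay it becomes the player's view target.
; Releasing W raises the mesh's Y by a fixed interval, while S lowers it only while the distance exceeds a minimum.
; UpdateDistance stores and prints the absolute Y gap between camera and mesh at startup and after each move.
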(event EventBeginPlay
  (Game|Player|SetViewTargetwithBlend (Game|GetPlayerController 0) self 0.0 "VTBlend_Linear" 0.0 false)
  (CallFunction|UpdateDistance))

(event Input|KeyboardEvents|W
  (params (Key :type Key%20Structure))
  (bind _landcruiser_cylinder002 (Variables|Default|Getlandcruiser_Cylinder002))
  (bind _returnvalue (Transformation|GetWorldLocation _landcruiser_cylinder002))
  (bind (_x _y _z) (Math|Vector|BreakVector _returnvalue))
  ;[1 1 1] Comment
  (:Released
    (Transformation|SetWorldLocation _landcruiser_cylinder002 (Math|Vector|MakeVector _x (+ _y (Variables|Default|GetMoveInterval)) _z) false false)
    (CallFunction|UpdateDistance)))

(event Input|KeyboardEvents|S
  (params (Key :type Key%20Structure))
  (bind _landcruiser_cylinder002 (Variables|Default|Getlandcruiser_Cylinder002))
  (bind _returnvalue (Transformation|GetWorldLocation _landcruiser_cylinder002))
  (bind (_x _y _z) (Math|Vector|BreakVector _returnvalue))
  ;[1 1 1] Comment
  (:Released
    ;;[1 1 1] Don't get too close
    (if (> (Variables|Default|GetdistanceFromCar) (Variables|Default|GetMinDist))
      (Transformation|SetWorldLocation _landcruiser_cylinder002 (Math|Vector|MakeVector _x (- _y (Variables|Default|GetMoveInterval)) _z) false false)
      (CallFunction|UpdateDistance))))

(fn ConstructionScript)

(fn UpdateDistance
  (Variables|Default|SetdistanceFromCar (Math|Float|Absolute(Float) (- (.Y (Math|Vector|BreakVector (Transformation|GetWorldLocation (Variables|Default|GetCamera)))) (.Y (Math|Vector|BreakVector (Transformation|GetWorldLocation (Variables|Default|Getlandcruiser_Cylinder002)))))))
  (Development|PrintString (Utilities|String|ToString(Float) (Variables|Default|GetdistanceFromCar))))